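; BP_DamageType_Default is a damage type that processes a hit on an actor and returns the damage to apply.
; Blocked hits return zero, while unblocked hits pass damage through unchanged.
; When both actors are valid and the hit is unblocked, it reads status effect info from the causer through a message call.
; It forwards that crowd control type, duration and launch strength to the damaged actor, with the causer's location as source.
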(fn ProcessDamage
  (params (DamagedActor :type Actor%20Object%20Reference) (Damage :type Float%20%28double-precision%29) (Blocked :type Boolean) (DamageCauser :type Actor%20Object%20Reference))
  (Utilities|IsValid DamagedActor
    (:Is%20Valid
      (Utilities|IsValid DamageCauser
        (:Is%20Valid
          (if (not Blocked)
            (bind (_duration _damage _crowdcontrol _cc_duration _launchstrength) (Class|BIAbility|GetStatusEffectInfo(Message) DamageCauser))
            (Class|BICrowdControl|ReceiveCrowdControl(Message) DamagedActor _crowdcontrol (Transformation|GetActorLocation DamageCauser) _cc_duration _launchstrength false)))
        (:Is%20Not%20Valid
          _)))
    (:Is%20Not%20Valid
      _))
  (return (select Blocked 0.0 Damage)))