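; Boss projectile ability that aims projectiles at yaw angles spread around a circle, or a multiple of it set by the ability's modifier.
; On BeginPlay it derives an angle step by dividing the truncated Modifier Y × 360 degrees by the spawn count.
; GetProjectileTransform places each projectile at the current boss mesh socket, with a world yaw of the current SpawnCount times that step, independent of boss facing.
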(event EventBeginPlay
  (|CallParentFunction)
  (Variables|Default|SetTempAngle (Math|Conversions|ToFloat(Integer) (/ (Math|Float|Truncate (* (.Y (Math|Vector|BreakVector (.Modifier (Utilities|Struct|BreakF_BossAbility (Variables|Default|GetAbilityInfo))))) 3.6e+02)) (Variables|Default|GetSpawnCount)))))

(event Collision|EventActorBeginOverlap
  (params (OtherActor :type Actor%20Object%20Reference)))

(event EventTick
  (params (DeltaSeconds :type Float%20%28single-precision%29)))

(fn ConstructionScript
  (|CallParentFunction))

(fn GetProjectileTransform
  (return (Math|Transform|MakeTransform (Transformation|GetSocketLocation (Variables|/Script/Engine.Character|GetMesh (Variables|Default|GetBossRef)) (Utilities|String|StringToName (Utilities|Array|Get(acopy) (Variables|Default|GetSpawnSockets) (Variables|Default|GetSocketIndex)))) (Math|Rotator|MakeRotator 0.0 0.0 (* (Variables|Default|GetSpawnCount) (Variables|Default|GetTempAngle))))))