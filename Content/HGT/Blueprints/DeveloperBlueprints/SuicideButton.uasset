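; SuicideButton is a developer interactable that damages the character who activates it, apparently to force a death.
; A trigger overlap sets ShowHintstrings on the ThirdPersonCharacter, shows the hint on the GameplayPC's HUD and records who triggered it.
; Leaving the trigger clears the flag, hint and stored character.
; StartInteraction applies fixed damage to the passed-in activator when CanActivate is true, without reading the stored character.
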(event OnComponentBeginOverlap(Trigger)
  (params (OverlappedComponent :type Primitive%20Component%20Object%20Reference) (OtherActor :type Actor%20Object%20Reference) (OtherComp :type Primitive%20Component%20Object%20Reference) (OtherBodyIndex :type Integer) (bFromSweep :type Boolean) (SweepResult :type Hit%20Result%20Structure%20%28by%20ref%29))
  ;[1 1 1] Starting Random Weapon Trigger Stuff
  (bind _asthird_person_character (Utilities|Casting|CastToThirdPersonCharacter OtherActor))
  ;;[1 1 1] Sets this variable inside Thirdperson to True which then dispatches back the start trap message.
  (Variables|/Game/HGT/Characters/BaseCharacter/ThirdPersonCharacter.ThirdPersonCharacter_C|SetShowHintstrings? _asthird_person_character true)
  (bind _asgameplay_pc (Utilities|Casting|CastToGameplayPC (Pawn|GetController _asthird_person_character)))
  (Utilities|IsValid (Variables|/Game/HGT/CoreBlueprints/Gameplay/GameplayPC.GameplayPC_C|GetHUDWidgetReference _asgameplay_pc)
    (:Is%20Valid
      (Default|SetHintstring (Variables|/Game/HGT/CoreBlueprints/Gameplay/GameplayPC.GameplayPC_C|GetHUDWidgetReference _asgameplay_pc) (Variables|Default|GetHintstring))
      (Variables|Default|SetPersonWhoTriggered _asthird_person_character))))

(event OnComponentEndOverlap(Trigger)
  (params (OverlappedComponent :type Primitive%20Component%20Object%20Reference) (OtherActor :type Actor%20Object%20Reference) (OtherComp :type Primitive%20Component%20Object%20Reference) (OtherBodyIndex :type Integer))
  ;[1 1 1] Starting Random Weapon Trigger Stuff
  (bind _asthird_person_character (Utilities|Casting|CastToThirdPersonCharacter OtherActor))
  (Variables|/Game/HGT/Characters/BaseCharacter/ThirdPersonCharacter.ThirdPersonCharacter_C|SetShowHintstrings? _asthird_person_character false)
  (bind _asgameplay_pc (Utilities|Casting|CastToGameplayPC (Pawn|GetController _asthird_person_character)))
  (Utilities|IsValid (Variables|/Game/HGT/CoreBlueprints/Gameplay/GameplayPC.GameplayPC_C|GetHUDWidgetReference _asgameplay_pc)
    (:Is%20Valid
      (Default|SetHintstring (Variables|/Game/HGT/CoreBlueprints/Gameplay/GameplayPC.GameplayPC_C|GetHUDWidgetReference _asgameplay_pc))
      (Variables|Default|SetPersonWhoTriggered 0))))

(event EventStartInteraction
  (params (CanActivate? :type Boolean) (PersonWhoActivatedIt :type Third%20Person%20Character%20Object%20Reference))
  ;[1 1 1] Starting Random Weapon Trigger Stuff
  (if CanActivate?
    (Game|Damage|ApplyDamage PersonWhoActivatedIt 2e+02 0 0)))

(fn ConstructionScript)