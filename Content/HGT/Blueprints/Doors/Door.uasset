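; Purchasable door that players open by spending points, activating new zones in the game mode.
; Overlapping the trigger shows a cost hint on the HUD, swaps the character's pickup time to the door's open time and caches affordability.
; A valid interaction wakes net dormancy, rechecks and deducts the player's points, activates the linked zones and destroys the door.
; Leaving the trigger clears the hint and restores the interaction time.
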(event OnComponentBeginOverlap(DoorTrigger)
  (params (OverlappedComponent :type Primitive%20Component%20Object%20Reference) (OtherActor :type Actor%20Object%20Reference) (OtherComp :type Primitive%20Component%20Object%20Reference) (OtherBodyIndex :type Integer) (bFromSweep :type Boolean) (SweepResult :type Hit%20Result%20Structure%20%28by%20ref%29))
  (bind _asthird_person_character (Utilities|Casting|CastToThirdPersonCharacter OtherActor))
  ;[1 1 1] Sets this variable inside Thirdperson to True which then dispatches back the start trap message.
  (Variables|/Game/HGT/Characters/BaseCharacter/ThirdPersonCharacter.ThirdPersonCharacter_C|SetShowHintstrings? _asthird_person_character true)
  (Variables|/Game/HGT/Characters/BaseCharacter/ThirdPersonCharacter.ThirdPersonCharacter_C|SetPickupTime _asthird_person_character (Variables|Default|GetOpenTime)) ; Reset Pickup Time back to normal
  (bind _asgameplay_pc (Utilities|Casting|CastToGameplayPC (Pawn|GetController _asthird_person_character)))
  (if (>= (Variables|/Game/HGT/CoreBlueprints/Gameplay/GameplayPC.GameplayPC_C|GetPoints _asgameplay_pc) (Variables|Default|GetCost))
    (Variables|Default|SetCanAfford? true)
    (else
      (Variables|Default|SetCanAfford? false)))
  (Utilities|IsValid (Variables|/Game/HGT/CoreBlueprints/Gameplay/GameplayPC.GameplayPC_C|GetHUDWidgetReference _asgameplay_pc)
    (:Is%20Valid
      (Default|SetHintstring (Variables|/Game/HGT/CoreBlueprints/Gameplay/GameplayPC.GameplayPC_C|GetHUDWidgetReference _asgameplay_pc) (Utilities|Text|ToText(String) (Utilities|String|Append (Utilities|String|ToString(Text) (Variables|Default|GetHintstring)) (Utilities|String|ToString(Integer) (Variables|Default|GetCost)) " Points"))))))

(event OnComponentEndOverlap(DoorTrigger)
  (params (OverlappedComponent :type Primitive%20Component%20Object%20Reference) (OtherActor :type Actor%20Object%20Reference) (OtherComp :type Primitive%20Component%20Object%20Reference) (OtherBodyIndex :type Integer))
  (bind _asthird_person_character (Utilities|Casting|CastToThirdPersonCharacter OtherActor))
  (Variables|/Game/HGT/Characters/BaseCharacter/ThirdPersonCharacter.ThirdPersonCharacter_C|SetShowHintstrings? _asthird_person_character false)
  (Variables|/Game/HGT/Characters/BaseCharacter/ThirdPersonCharacter.ThirdPersonCharacter_C|SetPickupTime _asthird_person_character (Variables|/Game/HGT/Characters/BaseCharacter/ThirdPersonCharacter.ThirdPersonCharacter_C|GetInteractionTime _asthird_person_character)) ; Reset Pickup Time back to normal
  (bind _asgameplay_pc (Utilities|Casting|CastToGameplayPC (Pawn|GetController _asthird_person_character)))
  (Utilities|IsValid (Variables|/Game/HGT/CoreBlueprints/Gameplay/GameplayPC.GameplayPC_C|GetHUDWidgetReference _asgameplay_pc)
    (:Is%20Valid
      (Default|SetHintstring (Variables|/Game/HGT/CoreBlueprints/Gameplay/GameplayPC.GameplayPC_C|GetHUDWidgetReference _asgameplay_pc)))))

(event Custom|OpenDoor
  (params (PersonWhoOpenedDoor :type Third%20Person%20Character%20Object%20Reference))
  (bind _output_get (Variables|Default|SetPersonWhoOpenedDoor PersonWhoOpenedDoor))
  (bind _asgameplay_pc (Utilities|Casting|CastToGameplayPC (Pawn|GetController _output_get)))
  (if (>= (Variables|/Game/HGT/CoreBlueprints/Gameplay/GameplayPC.GameplayPC_C|GetPoints _asgameplay_pc) (Variables|Default|GetCost)) ; Do You Have Enough Points?
    (Default|RemovePoints _asgameplay_pc (Variables|Default|GetCost))
    (bind _asgameplay_gm (Utilities|Casting|CastToGameplayGM (Game|GetGameMode)))
    (Default|ActivateNewZones _asgameplay_gm (Variables|Default|GetEnteredZoneToActivate))
    (Actor|DestroyActor)))

(event EventBeginPlay)

(event Collision|EventActorBeginOverlap
  (params (OtherActor :type Actor%20Object%20Reference)))

(event EventTick
  (params (DeltaSeconds :type Float%20%28single-precision%29)))

(event EventStartInteraction
  (params (CanActivate? :type Boolean) (PersonWhoActivatedIt :type Third%20Person%20Character%20Object%20Reference))
  (if CanActivate?
    (if (Variables|Default|GetCanAfford?)
      (Networking|SetNetDormancy "DORM_Never")
      (CallFunction|OpenDoor PersonWhoActivatedIt)
      (Variables|Default|SetCanAfford? false))))

(fn ConstructionScript)