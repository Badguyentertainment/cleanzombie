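; Base weapon Blueprint with separate first-person and third-person meshes for the owning player.
; Construction disables actor collision and makes first-person child components visible only to the owner.
; InitialWeaponEquip attaches each mesh to its socket on the player's arms or body, then toggles owner visibility on both meshes and their child components to match the current view.
; A separate event instantly stops montages on the first-person weapon to cancel reloads.
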(event Custom|StopReloadMontage
  (bind _fp_mesh (Variables|Default|GetFP_Mesh))
  (bind _returnvalue (Components|SkeletalMesh|GetAnimInstance _fp_mesh))
  ;[1 1 1] Stops The Reload Montage On The First Person Weapon
  (Utilities|IsValid _returnvalue
    (:Is%20Valid
      (Animation|Montage|MontageStop _returnvalue 0.0 0))))

(event EventInitialWeaponEquip
  (params (OwningPlayerREF :type Third%20Person%20Character%20Object%20Reference))
  ;[1 1 1] Attach Weapons to Correct Locations Depending On If It's a First Person or Third Person Weapon
  (Utilities|IsValid OwningPlayerREF
    (:Is%20Valid
      (Variables|Default|SetOwningPlayer_REF OwningPlayerREF)
      (Transformation|AttachComponentToComponent (Variables|Default|GetFP_Mesh) (Variables|/Game/HGT/Characters/BaseCharacter/ThirdPersonCharacter.ThirdPersonCharacter_C|GetFP_Arms OwningPlayerREF) (Variables|/Game/HGT/Characters/BaseCharacter/ThirdPersonCharacter.ThirdPersonCharacter_C|GetFP%20Weapon%20Socket OwningPlayerREF) "SnapToTarget" "SnapToTarget" "SnapToTarget" true)
      (Transformation|AttachComponentToComponent (Variables|Default|GetTP_Mesh) (Variables|/Script/Engine.Character|GetMesh OwningPlayerREF) (Variables|/Game/HGT/Characters/BaseCharacter/ThirdPersonCharacter.ThirdPersonCharacter_C|GetCWSocketName OwningPlayerREF) "SnapToTarget" "SnapToTarget" "SnapToTarget" true)
      (if (Variables|/Game/HGT/Characters/BaseCharacter/ThirdPersonCharacter.ThirdPersonCharacter_C|GetisInFirstPerson? (Variables|Default|GetOwningPlayer_REF))
        (Class|PrimitiveComponent|SetOwnerNoSee (Variables|Default|GetTP_Mesh) true) ; Hide TP Weapon
        (Class|PrimitiveComponent|SetOwnerNoSee (Variables|Default|GetFP_Mesh) false) ; Show FP Weapon
        ;[1 1 1] Get all 1st person Child Components and Show them if in 1st person
        (for _array_element (Components|GetChildrenComponents (Variables|Default|GetFP_Mesh) true)
          (bind _asprimitive_component (Utilities|Casting|CastToPrimitiveComponent _array_element))
          (Utilities|IsValid _asprimitive_component
            (:Is%20Valid
              (Class|PrimitiveComponent|SetOwnerNoSee _asprimitive_component false))))
        ;[1 1 1] Get all 3rd person components and Hide them when in 1st person
        (for _array_element_2 (Components|GetChildrenComponents (Variables|Default|GetTP_Mesh) true)
          (bind _asprimitive_component_2 (Utilities|Casting|CastToPrimitiveComponent _array_element_2))
          (Utilities|IsValid _asprimitive_component_2
            (:Is%20Valid
              (Class|PrimitiveComponent|SetOwnerNoSee _asprimitive_component_2 true))))
        (else
          (Class|PrimitiveComponent|SetOwnerNoSee (Variables|Default|GetTP_Mesh) false) ; Show TP Weapon
          (Class|PrimitiveComponent|SetOwnerNoSee (Variables|Default|GetFP_Mesh) true) ; Hide FP Weapon
          ;[1 1 1] Get all 1st person Child Components and Hide them if in 3rd person
          (for _array_element_3 (Components|GetChildrenComponents (Variables|Default|GetFP_Mesh) true)
            (bind _asprimitive_component_3 (Utilities|Casting|CastToPrimitiveComponent _array_element_3))
            (Utilities|IsValid _asprimitive_component_3
              (:Is%20Valid
                (Class|PrimitiveComponent|SetOwnerNoSee _asprimitive_component_3 true))))
          ;[1 1 1] Get all 3rd person components and show them when in 3rd person
          (for _array_element_4 (Components|GetChildrenComponents (Variables|Default|GetTP_Mesh) true)
            (bind _asprimitive_component_4 (Utilities|Casting|CastToPrimitiveComponent _array_element_4))
            (Utilities|IsValid _asprimitive_component_4
              (:Is%20Valid
                (Class|PrimitiveComponent|SetOwnerNoSee _asprimitive_component_4 false)))))))))

(fn ConstructionScript
  (Collision|SetActorEnableCollision false)
  (for _array_element (Components|GetChildrenComponents (Variables|Default|GetFP_Mesh) true)
    (bind _asprimitive_component (Utilities|Casting|CastToPrimitiveComponent _array_element))
    (Utilities|IsValid _asprimitive_component
      (:Is%20Valid
        (Rendering|SetOnlyOwnerSee _asprimitive_component true :!class /Script/Engine.PrimitiveComponent)))))