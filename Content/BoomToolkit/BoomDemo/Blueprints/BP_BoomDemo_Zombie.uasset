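; Demo zombie AI character for BoomToolkit that chases a randomly chosen player and damages it up close.
; BeginPlay randomizes its scale, body color and walk speed and picks the target.
; Tick issues AIMoveTo whenever it is stationary and out of range, while a sphere overlap runs a looping timer that applies damage.
; Incoming damage depletes health, and death ragdolls the mesh, disables capsule collision and sets a lifespan.
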(event OnComponentBeginOverlap(Sphere)
  (params (OverlappedComponent :type Primitive%20Component%20Object%20Reference) (OtherActor :type Actor%20Object%20Reference) (OtherComp :type Primitive%20Component%20Object%20Reference) (OtherBodyIndex :type Integer) (bFromSweep :type Boolean) (SweepResult :type Hit%20Result%20Structure%20%28by%20ref%29))
  ;[1 1 1] Demo AI logic.
  (if (== OtherActor (Variables|Default|GetTargetPlayer)) ; Is the overlapping actor the target player?
    (Utilities|Time|SetTimerbyFunctionName 0 "DamagePlayer" 1.0 true) ; Start damage cycle.
  ))

(event OnComponentEndOverlap(Sphere)
  (params (OverlappedComponent :type Primitive%20Component%20Object%20Reference) (OtherActor :type Actor%20Object%20Reference) (OtherComp :type Primitive%20Component%20Object%20Reference) (OtherBodyIndex :type Integer))
  ;[1 1 1] Demo AI logic.
  (if (== OtherActor (Variables|Default|GetTargetPlayer)) ; Is the nolonger overlapping actor the target player?
    (Utilities|Time|ClearTimerbyFunctionName 0 "DamagePlayer") ; Stop the damage cycle.
  ))

(event Custom|DamagePlayer
  ;[1 1 1] Demo AI logic.
  (Game|Damage|ApplyDamage (Variables|Default|GetTargetPlayer) 1e+01 0 0) ; Apply damage to target player.
)

(event Custom|KillAI
  ;[1 1 1] Demo AI logic.
  (Physics|SetSimulatePhysics (Variables|Character|GetMesh) true) ; Set AI mesh to simulate physics.
  (Class|PrimitiveComponent|WakeAllRigidBodies (Variables|Character|GetMesh)) ; Wake rigid bodies on AI mesh.
  (Collision|SetCollisionEnabled (Variables|Collision|GetCapsuleComponent) "NoCollision") ; Turn capsule collision off.
  (Actor|SetLifeSpan 1e+01) ; Set AI lifespan.
)

(event EventBeginPlay
  (bind _returnvalue (Math|Random|RandomUnitVector))
  (bind (_x _y _z) (Math|Vector|BreakVector _returnvalue))
  ;[1 1 1] Demo AI logic.
  (Transformation|SetActorScale3D (Math|Conversions|ToVector(Float) (Math|Random|RandomFloatinRange 0.35 1.65))) ; Randomize AI scaling.
  (bind _returnvalue_2 (Rendering|Material|CreateDynamicMaterialInstance (Variables|Character|GetMesh) 0 "/Game/BoomToolkit/BoomDemo/Materials/M_UE4Man_Body.M_UE4Man_Body" "None" :!class /Script/Engine.PrimitiveComponent)) ; Retrieve dynamic version of mesh material.
  (Rendering|Material|SetVectorParameterValue _returnvalue_2 "BodyColor" (Utilities|Struct|MakeLinearColor _x _y _z 0.0) :!class /Script/Engine.MaterialInstanceDynamic) ; Randomize AI mesh color.
  (bind _outactors (Actor|GetAllActorsOfClass "/Game/BoomToolkit/BoomDemo/Blueprints/Game/BP_BoomDemo_Character.BP_BoomDemo_Character_C")) ; Get a list of all players in the world.
  (Variables|Default|SetTargetPlayer (Utilities|Array|Get(acopy) _outactors (Math|Random|RandomIntegerinRange 0 (Utilities|Array|LastIndex _outactors)))) ; Select one at random and store for use.
  (Variables|/Script/Engine.CharacterMovementComponent|SetMaxWalkSpeed (Variables|Character|GetCharacterMovement) (Math|Random|RandomFloatinRange 2e+02 5e+02)) ; Give zombie randomized walk speed.
  (Variables|Default|SetStationary true) ; Set stationary to true.
)

(event EventTick
  (params (DeltaSeconds :type Float%20%28single-precision%29))
  ;[1 1 1] Demo AI logic.
  (if (not (Variables|Default|GetDead)) ; Is this AI dead?
    (if (Variables|Default|GetStationary) ; Is the AI currently stationary?
      (if (> (Transformation|GetDistanceTo (Variables|Default|GetTargetPlayer)) 2e+02) ; Is the target player more than 200 units away?
        (Variables|Default|SetStationary false) ; Clear stationary state.
        (AI|AIMoveTo (AI|GetAIController self) "0, 0, 0" (Variables|Default|GetTargetPlayer) -1.0 "Default" "Default" true true ; Move AI to target player.
          (:OnRequestFailed
            _)
          (:OnMoveFinished
            _))
        (Variables|Default|SetStationary true) ; Update stationary state.
      ))))

(event Game|Damage|EventAnyDamage
  (params (Damage :type Float%20%28single-precision%29) (DamageType :type Damage%20Type%20Object%20Reference) (InstigatedBy :type Controller%20Object%20Reference) (DamageCauser :type Actor%20Object%20Reference))
  ;[1 1 1] Demo AI logic.
  (bind _output_get (Variables|Default|SetHealth (- (Variables|Default|GetHealth) Damage))) ; Remove damage from AI health.
  (if (<= _output_get 0.0) ; Has the AI's health depleted?
    (Variables|Default|SetDead true) ; Update dead state.
    (Components|Movement|StopMovementImmediately (Variables|Character|GetCharacterMovement)) ; Stop AI movement.
    (CallFunction|KillAI) ; Run AI death event.
  ))

(fn ConstructionScript)