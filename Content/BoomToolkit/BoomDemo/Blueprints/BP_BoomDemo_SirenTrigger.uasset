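; One-shot trigger zone in the BoomToolkit demo that starts a repeating siren once the demo character enters it.
; The first overlap by a BP_BoomDemo_Character sets a Played flag, waits SirenDelay, then fades out that character's music track.
; It then plays the siren as a 2D sound and starts a looping timer that replays it every LoopSpeed interval, with no stop logic.
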(event OnComponentBeginOverlap(Zone)
  (params (OverlappedComponent :type Primitive%20Component%20Object%20Reference) (OtherActor :type Actor%20Object%20Reference) (OtherComp :type Primitive%20Component%20Object%20Reference) (OtherBodyIndex :type Integer) (bFromSweep :type Boolean) (SweepResult :type Hit%20Result%20Structure%20%28by%20ref%29))
  ;[1 1 1] Siren logic.
  (bind _asbp_boom_demo_character (Utilities|Casting|CastToBP_BoomDemo_Character OtherActor)) ; Is the overlapping actor a BoomDemo character?
  (if (not (Variables|Default|GetPlayed)) ; Has this already been played?
    (Variables|Default|SetPlayed true) ; Update played state.
    (Utilities|FlowControl|Delay (Variables|Default|GetSirenDelay)) ; Wait 22 seconds.
    (Audio|Components|Audio|FadeOut (Variables|/Game/BoomToolkit/BoomDemo/Blueprints/Game/BP_BoomDemo_Character.BP_BoomDemo_Character_C|GetMusicTrack _asbp_boom_demo_character) 5.0 0.0 "Linear" :!class /Script/Engine.AudioComponent) ; Fade out the ambient music.
    (CallFunction|SirenTimer) ; Trigger the initial siren.
    (Utilities|Time|SetTimerbyFunctionName 0 "SirenTimer" (Variables|Default|GetLoopSpeed) true) ; Start the siren timer loop.
  ))

(event Custom|SirenTimer
  ;[1 1 1] Siren logic.
  (Audio|PlaySound2D "/Game/BoomToolkit/BoomDemo/Audio/A_BoomDemo_Siren_Cue.A_BoomDemo_Siren_Cue" 1.0 1.0 0.0 0 0) ; Play the siren.
)

(fn ConstructionScript)