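; BP_BoomDemo_Arnie is a BoomToolkit demo mannequin that gives visual feedback when it takes damage.
; At BeginPlay, the UseText flag sets the visibility of its two text renders.
; AnyDamage writes the damage as a percentage to the second text render and creates a dynamic body material from M_UE4Man_Body.
; The body color turns red for a short delay, then changes to a fixed grey-tan, despite comments saying it is randomized.
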(event EventBeginPlay
  (Rendering|SetVisibility (Variables|Default|GetTextRender) (Variables|Default|GetUseText) false))

(event Game|Damage|EventAnyDamage
  (params (Damage :type Float%20%28single-precision%29) (DamageType :type Damage%20Type%20Object%20Reference) (InstigatedBy :type Controller%20Object%20Reference) (DamageCauser :type Actor%20Object%20Reference))
  (Rendering|Components|TextRender|SetText (Variables|Default|GetTextRender1) (Utilities|Text|ToText(String) (Utilities|String|Append (Utilities|String|ToString(Float) Damage) "%")))
  (bind _returnvalue (Rendering|Material|CreateDynamicMaterialInstance (Variables|Character|GetMesh) 0 "/Game/BoomToolkit/BoomDemo/Materials/M_UE4Man_Body.M_UE4Man_Body" "None" :!class /Script/Engine.PrimitiveComponent)) ; Retrieve dynamic version of mesh material.
  (Rendering|Material|SetVectorParameterValue _returnvalue "BodyColor" "(R=1.000000,G=0.000000,B=0.000000,A=1.000000)" :!class /Script/Engine.MaterialInstanceDynamic) ; Randomize AI mesh color.
  (Utilities|FlowControl|Delay 1.0)
  (Rendering|Material|SetVectorParameterValue _returnvalue "BodyColor" "(R=0.450786,G=0.407240,B=0.361307,A=0.000000)" :!class /Script/Engine.MaterialInstanceDynamic) ; Randomize AI mesh color.
)

(fn ConstructionScript)