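; First-person player character for the Boom Toolkit demo level, starting hidden with weapon actions disabled until SetEnabled.
; Authority-gated events handle hitscan fire, alt-fire projectiles and cycling of grenade and mine types, while F places surface-aligned land mines.
; Damage updates the HUD widget and starts delayed, timer-driven regen, with death possible only while enabled.
; E triggers the current example bomb, and HUD text shows weapon names and instructions.
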(event Custom|FireWeapon
  (params (WorldLocation :type Vector) (ForwardVector :type Vector))
  ;[0.5 1 0.5] Boom Demo Logic.
  (Networking|SwitchHasAuthority ; Ensure this only runs on the network\nauthority (server).
    (:Authority
      (bind _outhit (Collision|LineTraceByChannel WorldLocation (+ WorldLocation (* ForwardVector 5e+03)) "TraceTypeQuery1" false 0 "None" true "(R=1.000000,G=0.000000,B=0.000000,A=1.000000)" "(R=0.000000,G=1.000000,B=0.000000,A=1.000000)" 2.0)) ; Do a line trace from the camera to the middle of the screen\n5000 units away.
      (Utilities|IsValid (.HitActor (Collision|BreakHitResult _outhit)) ; Was an actor hit by the line trace?
        (:Is%20Valid
          (Game|Damage|ApplyDamage (.HitActor (Collision|BreakHitResult _outhit)) 2e+01 (Pawn|GetController) self) ; Apply damage to actor.
          (CallFunction|ImpactEffect (.Location (Collision|BreakHitResult _outhit))) ; Run ImpactEffect event, parsing hit location for use.
        )))))

(event Custom|SpawnProjectile
  (bind _returnvalue (Pawn|GetControlRotation :!class /Script/Engine.Pawn))
  (bind _self self)
  ;[0.5 1 0.5] Boom Demo Logic.
  (Networking|SwitchHasAuthority ; Ensure projectile only spawns on server.
    (:Authority
      (bind _returnvalue_2 (Game|SpawnActorfromClass (Variables|Data|GetCurrentProjectile) (Math|Transform|MakeTransform (+ (Transformation|GetActorLocation) (Math|Vector|RotateVector "150.000000,33.000000, 0" _returnvalue)) _returnvalue) "Undefined" "SelectDefaultAtRuntime" _self _self)) ; Spawn projectile actor at actor's location, offsetting a little to avoid collision.
      (Class|BPBoomIntExplosionActor|SetOwningPawn(Message) _returnvalue_2 self) ; Set owning pawn in projectile.
    )))

(event Custom|UpdateClientWeapon
  (params (Weapon :type Integer))
  ;[0.5 1 0.5] Boom Demo Logic.
  (if (Pawn|IsLocallyControlled) ; Ensure this only runs on the local player.
    (switch int Weapon ; Based on the current weapon integer...
      (:0
        (Variables|Data|SetWeaponName "Gas Impact Grenades") ; Set WeaponName.
      )
      (:1
        (Variables|Data|SetWeaponName "Bouncing Grenades (3 sec fuse)") ; Set WeaponName.
      )
      (:2
        (Variables|Data|SetWeaponName "Sticky Cluster Bomb (spawns sticky proxy bombs)") ; Set WeaponName.
      )
      (:3
        (Variables|Data|SetWeaponName "Sticky Proximity Mines") ; Set WeaponName.
      ))
    (Variables|/Game/BoomToolkit/BoomDemo/Blueprints/Game/BP_BoomDemo_HUD.BP_BoomDemo_HUD_C|SetCurrentWeapon (.AsBP%20Boom%20Demo%20HUD (Utilities|Casting|CastToBP_BoomDemo_HUD (HUD|GetHUD (Game|GetPlayerController 0)))) (Variables|Data|GetWeaponName)) ; Update CurrentWeapon string in demo HUD.
  ))

(event Custom|CycleWeapon
  ;[0.5 1 0.5] Boom Demo Logic.
  (Networking|SwitchHasAuthority ; Ensure weapon cycle happens on server end.
    (:Authority
      (Math|Integer|IncrementInt (Variables|Data|GetCurrentWeapon) ; Increment current weapon reference integer.
        (:%20%20
          (if (> (Variables|Data|GetCurrentWeapon) (- (Utilities|Array|Length (Variables|Data|GetProjectiles)) 1)) ; Does the current weapon integer exceed\nthe number of array elements?
            (Variables|Data|SetCurrentWeapon 0) ; Reset current weapon to zero (first\narray element).
          )
          (Variables|Data|SetCurrentProjectile (Utilities|Array|Get(acopy) (Variables|Data|GetProjectiles) (Variables|Data|GetCurrentWeapon))) ; Set the current projectile.
          (CallFunction|UpdateClientWeapon (Variables|Data|GetCurrentWeapon)) ; Run client weapon switch notify event.
        )))))

(event Custom|Example
  (bind _currentexamplebomb (Variables|Data|GetCurrentExampleBomb))
  ;[0.5 1 0.5] Boom Demo Logic.
  (Utilities|IsValid _currentexamplebomb ; Is the current example type valid?
    (:Is%20Valid
      (Default|RunExample _currentexamplebomb) ; Trigger this example's RunExample event.
    )))

(event Custom|ImpactEffect
  (params (Location :type Vector))
  ;[0.5 1 0.5] Boom Demo Logic.
  (Effects|SpawnEmitteratLocation "/Game/BoomToolkit/Particles/P_Boom_ImpactSparks.P_Boom_ImpactSparks" Location) ; Spawn spark particle effect at parsed location.
)

(event Custom|ResetUse
  ;[0.5 1 0.5] Boom Demo Logic.
  (Variables|Default|SetAltFireReady true) ; Update AltFireReady state.
)

(event Custom|Regen
  ;[0.5 1 0.5] Boom Demo Logic.
  (bind _output_get (Variables|Default|SetHealth (Math|Float|Clamp(Float) (+ (Variables|Default|GetHealth) 0.1) 0.0 1e+02))) ; Add small amount of health.
  (Class|BPIntBoomDemoExample|SetHealth(Message) (Variables|Default|GetHUD) (/ _output_get 1e+02)) ; Update HUD.
  (if (>= (Variables|Default|GetHealth) 1e+02) ; Has health recharged fully?
    (Utilities|Time|ClearTimerbyFunctionName 0 "Regen") ; Stop regeneration.
  ))

(event Game|Damage|EventAnyDamage
  (params (Damage :type Float%20%28single-precision%29) (DamageType :type Damage%20Type%20Object%20Reference) (InstigatedBy :type Controller%20Object%20Reference) (DamageCauser :type Actor%20Object%20Reference))
  ;[0.5 0.5 1] Character Control Events.
  (Utilities|Time|ClearTimerbyFunctionName 0 "Regen") ; Stop the health regen timer.
  (if (Variables|Data|GetEnabled) ; Is the player enabled?
    (Variables|Default|SetHealth (- (Variables|Default|GetHealth) Damage)) ; Update health. Allow death.
    (else
      (Variables|Default|SetHealth (Math|Float|Clamp(Float) (- (Variables|Default|GetHealth) Damage) 5.0 1e+02)) ; Clamp health between 5 and 100 and update.
    ))
  (Class|BPIntBoomDemoExample|SetHealth(Message) (Variables|Default|GetHUD) (/ (Variables|Default|GetHealth) 1e+02)) ; Update HUD.
  (if (<= (Variables|Default|GetHealth) 0.0) ; Should the player be dead?
    (Variables|Data|SetEnabled false) ; Disable the player.
    (Pawn|Components|CharacterMovement|DisableMovement (Variables|Character|GetCharacterMovement)) ; Disable player movement.
    (CallFunction|ToggleVisibility true) ; Set player meshes to hidden on startup\nfor demo level.
    (Class|BPIntBoomDemoExample|SetHealth(Message) (Variables|Default|GetHUD) 0.0) ; Force HUD to zero health.
    (else
      (Utilities|FlowControl|RetriggerableDelay 1.5) ; Run delay for health regen.
      (Utilities|Time|SetTimerbyFunctionName 0 "Regen" 0.015 true) ; Start up health regen again.
    )))

(event EventSetEnabled
  (params (NewState :type Boolean))
  ;[0.5 1 0.5] Boom Demo Logic.
  (bind _output_get (Variables|Data|SetEnabled NewState)) ; Update enabled state.
  (CallFunction|ToggleVisibility (not _output_get)) ; Toggle player visibility.
)

(event EventTriggerMessage
  (params (Message :type String))
  ;[0.5 1 0.5] Boom Demo Logic.
  (Variables|/Game/BoomToolkit/BoomDemo/Blueprints/Game/BP_BoomDemo_HUD.BP_BoomDemo_HUD_C|SetInstructionText (.AsBP%20Boom%20Demo%20HUD (Utilities|Casting|CastToBP_BoomDemo_HUD (HUD|GetHUD (Game|GetPlayerController 0)))) Message) ; Display instructions on HUD.
)

(event EventSetButton
  (params (Example :type BP%20Boom%20Demo%20Projectile%20Button%20Object%20Reference))
  (bind _returnvalue (Game|GetPlayerController 0))
  (bind _returnvalue_2 (HUD|GetHUD _returnvalue))
  (bind _asbp_boom_demo_hud (Utilities|Casting|CastToBP_BoomDemo_HUD _returnvalue_2))
  ;[0.5 1 0.5] Boom Demo Logic.
  (bind _output_get (Variables|Data|SetCurrentExampleBomb Example)) ; Update CurrentExampleBomb reference.
  (Utilities|IsValid _output_get ; Is the udpated reference a valid type?
    (:Is%20Valid
      (Variables|/Game/BoomToolkit/BoomDemo/Blueprints/Game/BP_BoomDemo_HUD.BP_BoomDemo_HUD_C|SetInstructionText _asbp_boom_demo_hud "Press E to fire example.") ; Display instructions on HUD.
    )
    (:Is%20Not%20Valid
      (Variables|/Game/BoomToolkit/BoomDemo/Blueprints/Game/BP_BoomDemo_HUD.BP_BoomDemo_HUD_C|SetInstructionText _asbp_boom_demo_hud "") ; Clear instructions on HUD.
    )))

(event EventSetDialogueManager
  (params (DialogueManager :type BP%20Boom%20Demo%20Dialogue%20Manager%20Object%20Reference))
  ;[0.5 1 0.5] Boom Demo Logic.
  (Variables|Default|SetCurrentDialogueActor DialogueManager) ; Update current DialogueActor.
)

(event EventBeginPlay
  ;[0.5 0.5 1] Character Control Events.
  (Variables|Data|SetEnabled false) ; Disable character actions on startup.
  (CallFunction|ToggleVisibility true) ; Set player meshes to hidden on startup\nfor demo level.
  (CallFunction|CycleWeapon) ; Perform initial weapon cycle.
  (bind _returnvalue (Audio|SpawnSound2D "/Game/BoomToolkit/BoomDemo/Audio/A_BoomDemo_Ambient_Cue.A_BoomDemo_Ambient_Cue" 0.5 1.0 0.0 0)) ; Spawn music track.
  (Variables|Data|SetMusicTrack _returnvalue) ; Update music track variable.
  (bind _returnvalue_2 (UserInterface|CreateWidget "/Game/BoomToolkit/BoomDemo/Blueprints/W_HUD.W_HUD_C"))
  (bind _output_get (Variables|Default|SetHUD _returnvalue_2))
  (UserInterface|Viewport|AddtoViewport _output_get 0))

(event Input|ActionEvents|InputActionJump
  (params (Key :type Key%20Structure))
  ;[0.5 0.5 1] Base input controls.
  (:Pressed
    (Character|Jump) ; Start jumping.
  )
  (:Released
    (Character|StopJumping) ; Stop jumping.
  ))

(event Input|ActionEvents|InputActionFire
  (params (Key :type Key%20Structure))
  ;[0.5 1 0.5] Auxiliary Controls.
  (:Pressed
    (Utilities|CheckPlayer ; Check if the player is allowed to do\nauxiliary actions.
      (:Enabled
        (CallFunction|FireGun) ; Fire weapon input logic.
      ))))

(event Input|AxisEvents|InputAxisTurn
  (params (AxisValue :type Float%20%28single-precision%29))
  ;[0.5 0.5 1] Base input controls.
  (Pawn|Input|AddControllerYawInput AxisValue) ; Turn based on mouse input.
)

(event Input|AxisEvents|InputAxisLookUp
  (params (AxisValue :type Float%20%28single-precision%29))
  ;[0.5 0.5 1] Base input controls.
  (Pawn|Input|AddControllerPitchInput AxisValue) ; Look up and down based on mouse input.
)

(event Input|AxisEvents|InputAxisMoveForward
  (params (AxisValue :type Float%20%28single-precision%29))
  ;[0.5 0.5 1] Base input controls.
  (Pawn|Input|AddMovementInput (Transformation|GetActorForwardVector) AxisValue false) ; Move character forward and back.
)

(event Input|AxisEvents|InputAxisMoveRight
  (params (AxisValue :type Float%20%28single-precision%29))
  ;[0.5 0.5 1] Base input controls.
  (Pawn|Input|AddMovementInput (Transformation|GetActorRightVector) AxisValue false) ; Strafe left and right.
)

(event Input|MouseEvents|RightMouseButton
  (params (Key :type Key%20Structure))
  ;[0.5 1 0.5] Auxiliary Controls.
  (:Pressed
    (if (Variables|Default|GetAltFireReady) ; Is alt fire ready?
      (Utilities|CheckPlayer ; Check if the player is allowed to do\nauxiliary actions.
        (:Enabled
          (Variables|Default|SetAltFireReady false) ; Clear alt fire ready state to prevent\nspamming.
          (Utilities|Time|SetTimerbyFunctionName 0 "ResetUse" 0.5) ; Reset alt fire ready state after 1 second.
          (Animation|Montage|MontagePlay (Components|SkeletalMesh|GetAnimInstance (Variables|CharacterBase|GetMesh2P)) "/Game/BoomToolkit/BoomDemo/Animations/M_BoomDemo_FPFireMontage.M_BoomDemo_FPFireMontage" 1.0 "MontageLength" 0.0 true) ; Play weapon fire animation.
          (Audio|PlaySoundatLocation "/Game/BoomToolkit/Audio/S_Boom_WeaponFire_Cue.S_Boom_WeaponFire_Cue" (Transformation|GetActorLocation) "0, 0, 0" 1.0 1.0 0.0 0 0 0 0) ; Play weapon fire sound.
          (CallFunction|SpawnProjectile) ; Trigger projectile spawn.
        )))))

(event Input|KeyboardEvents|Tab
  (params (Key :type Key%20Structure))
  ;[0.5 1 0.5] Auxiliary Controls.
  (:Pressed
    (CallFunction|CycleWeapon) ; Cycle through example weapons.
  ))

(event Input|KeyboardEvents|F
  (params (Key :type Key%20Structure))
  (bind _self self)
  (bind _firstpersoncamera (Variables|CharacterBase|GetFirstPersonCamera))
  (bind _returnvalue (Transformation|GetWorldLocation _firstpersoncamera))
  ;[0.5 1 0.5] Auxiliary Controls.
  (:Pressed
    (Utilities|CheckPlayer ; Check if the player is allowed to do\nauxiliary actions.
      (:Enabled
        (bind _outhit (Collision|LineTraceByChannel _returnvalue (+ _returnvalue (* (Math|Vector|GetForwardVector _firstpersoncamera) 3e+02)) "TraceTypeQuery1" false 0 "None")) ; Perform line trace to determine spawn point.
        (Game|SpawnActorfromClass "/Game/BoomToolkit/Blueprints/Examples/ExplosionActors/BP_Boom_ExplosionActor_LandMine.BP_Boom_ExplosionActor_LandMine_C" (Math|Transform|MakeTransform (+ (.Location (Collision|BreakHitResult _outhit)) (* (.Normal (Collision|BreakHitResult _outhit)) 1e+01)) (Math|Rotator|MakeRotfromZ (.Normal (Collision|BreakHitResult _outhit)))) "Undefined" "OverrideRootScale" 0 _self _self) ; Spawn actor at line trace  hit location, aligning rotation to\nensure it matches the surface it spawns on.
      ))))

(event Input|KeyboardEvents|E
  (params (Key :type Key%20Structure))
  ;[0.5 1 0.5] Auxiliary Controls.
  (:Pressed
    (CallFunction|Example) ; Trigger example.
  ))

(fn ConstructionScript
  (Transformation|AttachComponentToComponent (Variables|CharacterBase|GetFP_Gun) (Variables|CharacterBase|GetMesh2P) "GripPoint" "SnapToTarget" "SnapToTarget" "SnapToTarget" true))

(fn FireGun
  (bind _firstpersoncamera (Variables|CharacterBase|GetFirstPersonCamera))
  (Animation|Montage|MontagePlay (Components|SkeletalMesh|GetAnimInstance (Variables|CharacterBase|GetMesh2P)) "/Game/BoomToolkit/BoomDemo/Animations/M_BoomDemo_FPFireMontage.M_BoomDemo_FPFireMontage" 1.0 "MontageLength" 0.0 true) ; Play weapon fire animation.
  (Audio|PlaySoundatLocation "/Game/BoomToolkit/Audio/S_Boom_WeaponFire.S_Boom_WeaponFire" (Transformation|GetActorLocation) "0, 0, 0" 1.0 1.0 0.0 0 0 0 0) ; Play weapon fire sound.
  (CallFunction|FireWeapon (Transformation|GetWorldLocation _firstpersoncamera) (Math|Vector|GetForwardVector _firstpersoncamera)) ; Trigger fire weapon event on the server.
  (return) ; Done.
)

(fn ToggleVisibility
  (params (NewHidden :type Boolean))
  (Development|SetHiddeninGame (Variables|Character|GetMesh) NewHidden false) ; Update player/gun mesh visibility based\non input.
  (return))

(fn GetDialogueManager
  (return (Variables|Default|GetCurrentDialogueActor)))