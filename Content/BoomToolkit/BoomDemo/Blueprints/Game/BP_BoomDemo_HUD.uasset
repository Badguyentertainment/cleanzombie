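; BP_BoomDemo_HUD is the example HUD for the Boom Toolkit demo, drawn immediate-mode in DrawHUD.
; When InstructionText is set, it draws that text centered near the bottom over a translucent box sized from the measured text.
; While the player BP_BoomDemo_Character has Enabled set, it also draws a center crosshair and a control hint that includes the CurrentWeapon name.
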(event EventDrawHUD
  (params (SizeX :type Integer) (SizeY :type Integer))
  (bind _instructiontext (Variables|Data|GetInstructionText))
  (bind (_outwidth _outheight) (Class|HUD|GetTextSize _instructiontext 0 1.25))
  ;[1 1 1] Example HUD logic.
  (Variables|Data|SetXVal SizeX) ; Store current SizeX for cleaner use.
  (Variables|Data|SetYVal SizeY) ; Store current SizeY for cleaner use.
  (if (> (Utilities|String|Len (Variables|Data|GetInstructionText)) 0) ; Is there currently an instruction text?
    (HUD|DrawRect "(R=1.000000,G=1.000000,B=1.000000,A=0.750000)" (- (Math|Conversions|ToFloat(Integer) (- (/ (Variables|Data|GetXVal) 2) (Math|Float|Truncate (/ (.OutWidth (Class|HUD|GetTextSize (Variables|Data|GetInstructionText) 0 1.25)) 2.0)))) 1e+01) (- (Math|Conversions|ToFloat(Integer) (- (Variables|Data|GetYVal) 100)) 5.0) (+ _outwidth 2e+01) (+ _outheight 1e+01)) ; Draw the text border.
    (HUD|DrawText (Variables|Data|GetInstructionText) "(R=0.009436,G=0.048327,B=0.165000,A=1.000000)" (Math|Conversions|ToFloat(Integer) (- (/ (Variables|Data|GetXVal) 2) (Math|Float|Truncate (/ (.OutWidth (Class|HUD|GetTextSize (Variables|Data|GetInstructionText) 0 1.25)) 2.0)))) (Math|Conversions|ToFloat(Integer) (- (Variables|Data|GetYVal) 100)) 0 1.25 false) ; Draw text telling player what alternate weapon is equipped.
  )
  (if (Variables|/Game/BoomToolkit/BoomDemo/Blueprints/Game/BP_BoomDemo_Character.BP_BoomDemo_Character_C|GetEnabled (.AsBP%20Boom%20Demo%20Character (Utilities|Casting|CastToBP_BoomDemo_Character (Game|GetPlayerCharacter 0)))) ; Is the player weapon enabled?
    (Canvas|DrawTexture "/Game/BoomToolkit/Textures/T_Boom_HUD_Crosshair.T_Boom_HUD_Crosshair" (Math|Conversions|ToFloat(Integer) (- (/ (Variables|Data|GetXVal) 2) 8)) (Math|Conversions|ToFloat(Integer) (- (/ (Variables|Data|GetYVal) 2) 8)) 16.0 16.0 0.0 0.0 1.0 1.0 (Utilities|Struct|MakeLinearColor 1.0 1.0 1.0 1.0) "BLEND_Translucent" 1.0 true) ; Draw crosshair in center of screen
    (HUD|DrawText (Utilities|String|Append "Left Mouse: Fire Instant Shot 
Right Mouse: " (Variables|Data|GetCurrentWeapon) " 
Press Tab to cycle alternate weapons. 
F to place a mine") "(R=1.000000,G=1.000000,B=1.000000,A=1.000000)" 3e+01 (Math|Conversions|ToFloat(Integer) (- (Variables|Data|GetYVal) 150)) 0 1.25 false) ; Draw text telling player what alternate weapon is equipped.
  ))

(fn ConstructionScript)