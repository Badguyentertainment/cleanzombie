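; BP_BoomDemo_Door is a two-panel sliding door for the Boom demo, with OpenDoor and CloseDoor events.
; Each event plays a 2D sound, updates the Open flag and slides both panels in opposite directions with MoveComponentTo, using offsets from their current positions.
; The trigger box only closes an open door on overlap; nothing in this graph calls OpenDoor.
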(event OnComponentBeginOverlap(Box)
  (params (OverlappedComponent :type Primitive%20Component%20Object%20Reference) (OtherActor :type Actor%20Object%20Reference) (OtherComp :type Primitive%20Component%20Object%20Reference) (OtherBodyIndex :type Integer) (bFromSweep :type Boolean) (SweepResult :type Hit%20Result%20Structure%20%28by%20ref%29))
  ;[1 1 1] Trigger overlap logic.
  (if (Variables|Default|GetOpen) ; Is this door open?
    (CallFunction|CloseDoor) ; Close the door.
  ))

(event Custom|CloseDoor
  (bind _rightdoor (Variables|Default|GetRightDoor))
  (bind _leftdoor (Variables|Default|GetLeftDoor))
  ;[1 1 1] Door close logic.
  (Utilities|FlowControl|Sequence ; Do these in order...
    (:then_0
      (Audio|PlaySound2D "/Game/BoomToolkit/BoomDemo/Audio/A_BoomDemo_Door_Cue.A_BoomDemo_Door_Cue" 1.0 1.0 0.0 0 0) ; Play door sound.
      (Variables|Default|SetOpen false) ; Update open state.
    )
    (:then_1
      (Components|MoveComponentTo _rightdoor (+ (Variables|/Script/Engine.SceneComponent|GetRelativeLocation _rightdoor) "-200.000000, 0, 0") (Variables|/Script/Engine.SceneComponent|GetRelativeRotation _rightdoor) false false 0.35 false) ; Close the right door.
    )
    (:then_2
      (Components|MoveComponentTo _leftdoor (+ (Variables|/Script/Engine.SceneComponent|GetRelativeLocation _leftdoor) "200.000000, 0, 0") (Variables|/Script/Engine.SceneComponent|GetRelativeRotation _leftdoor) false false 0.35 false) ; Close the left door.
    )))

(event Custom|OpenDoor
  (bind _rightdoor (Variables|Default|GetRightDoor))
  (bind _leftdoor (Variables|Default|GetLeftDoor))
  ;[1 1 1] Door open logic.
  (Utilities|FlowControl|Sequence
    (:then_0
      (Audio|PlaySound2D "/Game/BoomToolkit/BoomDemo/Audio/A_BoomDemo_Door_Cue.A_BoomDemo_Door_Cue" 1.0 1.0 0.0 0 0) ; Play door sound.
      (Variables|Default|SetOpen true) ; Update open state.
    )
    (:then_1
      (Components|MoveComponentTo _rightdoor (+ (Variables|/Script/Engine.SceneComponent|GetRelativeLocation _rightdoor) "200.000000, 0, 0") (Variables|/Script/Engine.SceneComponent|GetRelativeRotation _rightdoor) false false 0.35 false) ; Close the right door.
    )
    (:then_2
      (Components|MoveComponentTo _leftdoor (+ (Variables|/Script/Engine.SceneComponent|GetRelativeLocation _leftdoor) "-200.000000, 0, 0") (Variables|/Script/Engine.SceneComponent|GetRelativeRotation _leftdoor) false false 0.35 false) ; Close the left door.
    )))

(fn ConstructionScript)