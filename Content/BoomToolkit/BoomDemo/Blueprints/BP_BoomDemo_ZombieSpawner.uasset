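; Demo zombie spawner actor that periodically spawns AI-controlled BP_BoomDemo_Zombie pawns at its own location and rotation.
; While Enabled, Tick counts all zombie actors in the world and proceeds only when there are fewer than 120.
; A random Delay of a few seconds or less on the Tick path paces spawning, since the latent node ignores retriggers while pending.
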(event EventTick
  (params (DeltaSeconds :type Float%20%28single-precision%29))
  ;[1 1 1] Spawn zombies.
  (if (Variables|Default|GetEnabled) ; Is this spawner enabled?
    (bind _outactors (Actor|GetAllActorsOfClass "/Game/BoomToolkit/BoomDemo/Blueprints/BP_BoomDemo_Zombie.BP_BoomDemo_Zombie_C")) ; Get a list of all zombies...
    (if (not (>= (Utilities|Array|Length _outactors) 120)) ; Limit to 120 zombie actors.
      (Utilities|FlowControl|Delay (Math|Random|RandomFloatinRange 0.5 3.0)) ; Wait one second.
      (AI|SpawnAIFromClass "/Game/BoomToolkit/BoomDemo/Blueprints/BP_BoomDemo_Zombie.BP_BoomDemo_Zombie_C" 0 (Transformation|GetActorLocation) (Transformation|GetActorRotation) false 0) ; Spawn zombie AI.
    )))

(fn ConstructionScript)