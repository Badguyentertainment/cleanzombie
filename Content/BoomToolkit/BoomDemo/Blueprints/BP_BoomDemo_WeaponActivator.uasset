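; BP_BoomDemo_WeaponActivator is a trigger volume that switches the demo player's weapon and zombie spawning on and off.
; When a BP_BoomDemo_Character enters the Box, it enables that character's weapon via SetEnabledMessage and sets Enabled on every BP_BoomDemo_ZombieSpawner found with GetAllActorsOfClass.
; Leaving the box reverses both, disabling the weapon and all spawners.
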(event OnComponentBeginOverlap(Box)
  (params (OverlappedComponent :type Primitive%20Component%20Object%20Reference) (OtherActor :type Actor%20Object%20Reference) (OtherComp :type Primitive%20Component%20Object%20Reference) (OtherBodyIndex :type Integer) (bFromSweep :type Boolean) (SweepResult :type Hit%20Result%20Structure%20%28by%20ref%29))
  ;[1 1 1] Toggle weapon and zombie spawner states based on player entering/exiting volume.
  (bind _asbp_boom_demo_character (Utilities|Casting|CastToBP_BoomDemo_Character OtherActor)) ; Ensure this logic only runs on BP_BoomDemo_Character class.
  (Class|BPIntBoomDemoExample|SetEnabled(Message) _asbp_boom_demo_character true) ; Enable weapon on player.
  (bind _outactors (Actor|GetAllActorsOfClass "/Game/BoomToolkit/BoomDemo/Blueprints/BP_BoomDemo_ZombieSpawner.BP_BoomDemo_ZombieSpawner_C")) ; Retrieve a list of all zombie spawners...
  (for _array_element _outactors ; For each zombie spawner...
    (Variables|/Game/BoomToolkit/BoomDemo/Blueprints/BP_BoomDemo_ZombieSpawner.BP_BoomDemo_ZombieSpawner_C|SetEnabled _array_element true) ; Enable this zombie spawner.
  ))

(event OnComponentEndOverlap(Box)
  (params (OverlappedComponent :type Primitive%20Component%20Object%20Reference) (OtherActor :type Actor%20Object%20Reference) (OtherComp :type Primitive%20Component%20Object%20Reference) (OtherBodyIndex :type Integer))
  ;[1 1 1] Toggle weapon and zombie spawner states based on player entering/exiting volume.
  (bind _asbp_boom_demo_character (Utilities|Casting|CastToBP_BoomDemo_Character OtherActor)) ; Ensure this logic only runs on BP_BoomDemo_Character class.
  (Class|BPIntBoomDemoExample|SetEnabled(Message) _asbp_boom_demo_character false) ; Disable weapon on player.
  (bind _outactors (Actor|GetAllActorsOfClass "/Game/BoomToolkit/BoomDemo/Blueprints/BP_BoomDemo_ZombieSpawner.BP_BoomDemo_ZombieSpawner_C")) ; Retrieve a list of all zombie spawners...
  (for _array_element _outactors ; For each zombie spawner...
    (Variables|/Game/BoomToolkit/BoomDemo/Blueprints/BP_BoomDemo_ZombieSpawner.BP_BoomDemo_ZombieSpawner_C|SetEnabled _array_element false) ; Disable this zombie spawner.
  ))

(fn ConstructionScript)