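; Professor actor for the BoomToolkit demo that delivers a one-time scripted briefing when a player enters its detection volume, then opens its assigned door.
; Overlapping actors implementing BPInt_BoomDemo_Example receive timed subtitle messages, paired with mumble sound cues and sequenced by Delay nodes.
; The SecondInstance flag swaps the intro for an escape-emergency speech, which also clears the first siren trigger's timer and starts battle music.
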(event OnComponentBeginOverlap(PlayerDetection)
  (params (OverlappedComponent :type Primitive%20Component%20Object%20Reference) (OtherActor :type Actor%20Object%20Reference) (OtherComp :type Primitive%20Component%20Object%20Reference) (OtherBodyIndex :type Integer) (bFromSweep :type Boolean) (SweepResult :type Hit%20Result%20Structure%20%28by%20ref%29))
  ;[1 1 1] Professor discussion logic.
  (if (Utilities|DoesObjectImplementInterface OtherActor "/Game/BoomToolkit/BoomDemo/Blueprints/Game/BPInt_BoomDemo_Example.BPInt_BoomDemo_Example_C") ; Does the overlapping actor implement\nthe BPInt_BoomDemo_Example\ninterface?
    (if (not (Variables|Default|GetHasSpoken)) ; Has the professor already spoken?
      (Variables|Default|SetHasSpoken true) ; Update has spoken state.
      (Variables|Default|SetActor OtherActor) ; Store reference to overlapping actor\nfor use.
      (if (Variables|Default|GetSecondInstance) ; Is this the second instance of the professor?
        (Class|BPIntBoomDemoExample|TriggerMessage(Message) (Variables|Default|GetActor) "I'm afraid we're going to have to cut this short...") ; Trigger message.
        (Audio|PlaySound2D "/Game/BoomToolkit/BoomDemo/Audio/Dialogue/Clean/A_BoomDemo_Mumble04_Cue.A_BoomDemo_Mumble04_Cue" 1.0 1.0 0.0 0 0) ; Play "dialogue".
        (Utilities|FlowControl|Delay 3.0) ; Wait 3 seconds...
        (Class|BPIntBoomDemoExample|TriggerMessage(Message) (Variables|Default|GetActor) "It would appear the... subjects have managed to escape.") ; Trigger message.
        (Audio|PlaySound2D "/Game/BoomToolkit/BoomDemo/Audio/Dialogue/Clean/A_BoomDemo_Mumble05_Cue.A_BoomDemo_Mumble05_Cue" 1.0 1.0 0.0 0 0) ; Play "dialogue".
        (Utilities|FlowControl|Delay 3.0) ; Wait 3 seconds...
        (Class|BPIntBoomDemoExample|TriggerMessage(Message) (Variables|Default|GetActor) "There's a lot more we haven't covered... but... no time!") ; Trigger message.
        (Audio|PlaySound2D "/Game/BoomToolkit/BoomDemo/Audio/Dialogue/Clean/A_BoomDemo_Mumble08_Cue.A_BoomDemo_Mumble08_Cue" 1.0 1.0 0.0 0 0) ; Play "dialogue".
        (Utilities|FlowControl|Delay 2.0) ; Wait 3 seconds...
        (Class|BPIntBoomDemoExample|TriggerMessage(Message) (Variables|Default|GetActor) "We need you out there. You can use this new tech to...") ; Trigger message.
        (Audio|PlaySound2D "/Game/BoomToolkit/BoomDemo/Audio/Dialogue/Clean/A_BoomDemo_Mumble01_Cue.A_BoomDemo_Mumble01_Cue" 1.0 1.0 0.0 0 0) ; Play "dialogue".
        (Utilities|FlowControl|Delay 3.0) ; Wait 3 seconds...
        (Class|BPIntBoomDemoExample|TriggerMessage(Message) (Variables|Default|GetActor) "...resolve the situation. We will drop in some assistance when we can!") ; Trigger message.
        (Audio|PlaySound2D "/Game/BoomToolkit/BoomDemo/Audio/Dialogue/Clean/A_BoomDemo_Mumble05_Cue.A_BoomDemo_Mumble05_Cue" 1.0 1.0 0.0 0 0) ; Play "dialogue".
        (Utilities|FlowControl|Delay 3.0) ; Wait 2 seconds...
        (Class|BPIntBoomDemoExample|TriggerMessage(Message) (Variables|Default|GetActor)) ; Clear message.
        (Default|OpenDoor (Variables|Default|GetDoorActor)) ; Open the door assigned.
        (bind _outactors (Actor|GetAllActorsOfClass "/Game/BoomToolkit/BoomDemo/Blueprints/BP_BoomDemo_SirenTrigger.BP_BoomDemo_SirenTrigger_C")) ; Get all instances of the siren trigger.
        (Utilities|Time|ClearTimerbyFunctionName (Utilities|Array|Get(acopy) _outactors) "SirenTimer") ; Stop siren timer loop.
        (Audio|PlaySound2D "/Game/BoomToolkit/BoomDemo/Audio/A_BoomDemo_Battle_Cue.A_BoomDemo_Battle_Cue" 1.0 1.0 0.0 0 0) ; Trigger battle music.
        (else
          (Class|BPIntBoomDemoExample|TriggerMessage(Message) (Variables|Default|GetActor) "Ah good, you're here!... Running late again I see!") ; Trigger message.
          (Audio|PlaySound2D "/Game/BoomToolkit/BoomDemo/Audio/Dialogue/Clean/A_BoomDemo_Mumble01_Cue.A_BoomDemo_Mumble01_Cue" 1.0 1.0 0.0 0 0) ; Play "dialogue".
          (Utilities|FlowControl|Delay 2.0) ; Wait 2 seconds...
          (Class|BPIntBoomDemoExample|TriggerMessage(Message) (Variables|Default|GetActor) "We've got a new one for you to test today...") ; Trigger message.
          (Audio|PlaySound2D "/Game/BoomToolkit/BoomDemo/Audio/Dialogue/Clean/A_BoomDemo_Mumble06_Cue.A_BoomDemo_Mumble06_Cue" 1.0 1.0 0.0 0 0) ; Play "dialogue".
          (Utilities|FlowControl|Delay 2.0) ; Wait 2 seconds...
          (Class|BPIntBoomDemoExample|TriggerMessage(Message) (Variables|Default|GetActor) "We've developed a brand new technology that allows us to blow up ANYTHING!") ; Trigger message.
          (Audio|PlaySound2D "/Game/BoomToolkit/BoomDemo/Audio/Dialogue/Clean/A_BoomDemo_Mumble08_Cue.A_BoomDemo_Mumble08_Cue" 1.0 1.0 0.0 0 0) ; Play "dialogue".
          (Utilities|FlowControl|Delay 3.0) ; Wait 3 seconds...
          (Class|BPIntBoomDemoExample|TriggerMessage(Message) (Variables|Default|GetActor) "*mumbling* ...just think how good the next Ninja Turtles movie will be with this...") ; Trigger message.
          (Audio|PlaySound2D "/Game/BoomToolkit/BoomDemo/Audio/Dialogue/Clean/A_BoomDemo_Mumble04_Cue.A_BoomDemo_Mumble04_Cue" 1.0 1.0 0.0 0 0) ; Play "dialogue".
          (Utilities|FlowControl|Delay 3.0) ; Wait 3 seconds...
          (Class|BPIntBoomDemoExample|TriggerMessage(Message) (Variables|Default|GetActor) "*clears throat* Uh... I mean... let's get to testing... You will be experimenting with") ; Trigger message.
          (Audio|PlaySound2D "/Game/BoomToolkit/BoomDemo/Audio/Dialogue/Clean/A_BoomDemo_ClearThroat_Cue.A_BoomDemo_ClearThroat_Cue" 1.0 1.0 0.0 0 0) ; Play "dialogue".
          (Utilities|FlowControl|Delay 0.5) ; Wait 0.5 seconds...
          (Audio|PlaySound2D "/Game/BoomToolkit/BoomDemo/Audio/Dialogue/Clean/A_BoomDemo_Mumble07_Cue.A_BoomDemo_Mumble07_Cue" 1.0 1.0 0.0 0 0) ; Play "dialogue".
          (Utilities|FlowControl|Delay 3.0) ; Wait 1.5 seconds...
          (Class|BPIntBoomDemoExample|TriggerMessage(Message) (Variables|Default|GetActor) "two main types of explosives, though the new technology honestly allows us to make a lot more!") ; Trigger message.
          (Audio|PlaySound2D "/Game/BoomToolkit/BoomDemo/Audio/Dialogue/Clean/A_BoomDemo_Mumble05_Cue.A_BoomDemo_Mumble05_Cue" 1.0 1.0 0.0 0 0) ; Play "dialogue".
          (Utilities|FlowControl|Delay 3.0) ; Wait 3 seconds...
          (Class|BPIntBoomDemoExample|TriggerMessage(Message) (Variables|Default|GetActor) "Okay let's get started. Be sure to pay attention... I have a feeling we may need this technology") ; Trigger message.
          (Audio|PlaySound2D "/Game/BoomToolkit/BoomDemo/Audio/Dialogue/Clean/A_BoomDemo_Mumble08_Cue.A_BoomDemo_Mumble08_Cue" 1.0 1.0 0.0 0 0) ; Play "dialogue".
          (Utilities|FlowControl|Delay 3.0) ; Wait 3 seconds...
          (Class|BPIntBoomDemoExample|TriggerMessage(Message) (Variables|Default|GetActor) "sooner than we expect!") ; Trigger message.
          (Audio|PlaySound2D "/Game/BoomToolkit/BoomDemo/Audio/Dialogue/Clean/A_BoomDemo_Mumble06_Cue.A_BoomDemo_Mumble06_Cue" 1.0 1.0 0.0 0 0) ; Play "dialogue".
          (Utilities|FlowControl|Delay 2.0) ; Wait 2 seconds...
          (Class|BPIntBoomDemoExample|TriggerMessage(Message) (Variables|Default|GetActor)) ; Clear message.
          (Default|OpenDoor (Variables|Default|GetDoorActor)) ; Open door assigned to this instance.
        )))))

(fn ConstructionScript)