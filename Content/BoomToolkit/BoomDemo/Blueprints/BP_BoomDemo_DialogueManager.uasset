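; Trigger-zone dialogue manager for the Boom demo that plays a one-shot sequence of 2D voice tracks with on-screen messages.
; On first character overlap it registers itself as that character's current dialogue manager, then loops through parallel track, message and delay arrays.
; Before each step it checks that it is still current, so a newer manager cuts it short.
; When finished or superseded it opens an optional linked door, clearing the message only on completion.
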(event OnComponentBeginOverlap(Zone)
  (params (OverlappedComponent :type Primitive%20Component%20Object%20Reference) (OtherActor :type Actor%20Object%20Reference) (OtherComp :type Primitive%20Component%20Object%20Reference) (OtherBodyIndex :type Integer) (bFromSweep :type Boolean) (SweepResult :type Hit%20Result%20Structure%20%28by%20ref%29))
  (bind _door (Variables|Default|GetDoor))
  (bind _ascharacter (Utilities|Casting|CastToCharacter OtherActor)) ; Ensure overlapping actor is a character type.
  (Variables|Default|SetActor _ascharacter) ; Store overlapping actor for use.
  (if (not (Variables|Default|GetPlayed)) ; Has this already been played?
    (Variables|Default|SetPlayed true) ; Update played state.
    (Class|BPIntBoomDemoExample|SetDialogueManager(Message) (Variables|Default|GetActor) self) ; Update character dialogue manager reference.
    (bind _dialoguemanager (Class|BPIntBoomDemoExample|GetDialogueManager(Message) (Variables|Default|GetActor) :!label _label)) ; Get the character's current dialogue manager.
    (if (!= _dialoguemanager self) ; Is the player's current dialogue manager no longer this actor?
      _
      (else
        (bind _result (Math|Integer|IncrementInt (Variables|Default|GetCurrentTrack)) ; Increment current track value.
          (:%20%20
            (if (== _result (Utilities|Array|Length (Variables|Default|GetDialogueTracks))) ; Has the final dialogue been played?
              (Class|BPIntBoomDemoExample|TriggerMessage(Message) (Variables|Default|GetActor)) ; Clear message.
              (else
                (Audio|PlaySound2D (Utilities|Array|Get(acopy) (Variables|Default|GetDialogueTracks) (Variables|Default|GetCurrentTrack)) 1.0 1.0 0.0 0 0) ; Play the appropriate dialogue track.
                (Class|BPIntBoomDemoExample|TriggerMessage(Message) (Variables|Default|GetActor) (Utilities|Array|Get(acopy) (Variables|Default|GetMessages) (Variables|Default|GetCurrentTrack))) ; Triggere dialogue message.
                (Utilities|FlowControl|Delay (Utilities|Array|Get(acopy) (Variables|Default|GetDelayBetween) (Variables|Default|GetCurrentTrack))) ; Wait...
                (goto _label)))))))
    (Utilities|IsValid _door ; Is there a valid door reference?
      (:Is%20Valid
        (Default|OpenDoor _door) ; Open the door.
      ))))

(fn ConstructionScript)