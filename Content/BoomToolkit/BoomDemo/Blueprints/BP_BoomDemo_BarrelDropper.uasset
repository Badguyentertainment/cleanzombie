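; Demo dropper that rains batches of explosive assistance actors from the top of a box volume, owned and instigated by the player pawn.
; The first run drops the default class immediately; later runs wait randomly, play a radio line with an on-screen countdown, then pick a random class.
; Each batch spawns at random downward-facing points with physics enabled and is polled every few seconds until all are gone, restarting the cycle.
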(event EventBeginPlay
  (bind _returnvalue (Game|Player|GetPlayerPawn 0))
  (bind _returnvalue_2 (Game|Player|GetPlayerPawn 0))
  ;[1 1 1] Explosive actor spawning logic (for demo).
  (if (Variables|Default|GetFirstRun) ; Is it the first time that this logic has\nbeen executed?
    (Variables|Default|SetFirstRun false) ; Clear first run state.
    (Utilities|Array|Clear (Variables|Default|GetActiveActors) :!label _label) ; Clear active actors array.
    (for _index (range 1 (Math|Random|RandomIntegerinRange 2 8)) ; Run a random amount of times (between 2 and 8)...
      (bind _returnvalue_3 (Game|SpawnActorfromClass (Variables|Default|GetCurrentAssitance) (CallFunction|BuildTransform) "Undefined" "OverrideRootScale" _returnvalue _returnvalue _returnvalue)) ; Spawn explosive actor.
      (Physics|SetSimulatePhysics (Variables|/Game/BoomToolkit/Blueprints/BP_Boom_ExplosionActor.BP_Boom_ExplosionActor_C|GetBaseMesh _returnvalue_3) true) ; Ensure the explosion actor is set to simulate physics to allow\nit to fall instead of hovering in the air.
      (Utilities|Array|Add (Variables|Default|GetActiveActors) _returnvalue_3) ; Add this actor to the ActiveActors array for tracking.
    )
    (Utilities|FlowControl|Delay 3.0 :!label _label_2) ; Wait 3 seconds before rechecking active\nactors.
    (Variables|Default|SetReadyForReset true) ; Set ready for reset to true.
    (for _array_element (Variables|Default|GetActiveActors) ; For every active actor...
      (Utilities|IsValid _array_element ; Is the reference still valid?
        (:Is%20Valid
          (Variables|Default|SetReadyForReset false) ; As there is still an active actor, clear ready for reset state.
        )))
    (if (Variables|Default|GetReadyForReset) ; Is the system ready to be reset?
      (Utilities|FlowControl|Delay (Math|Random|RandomFloatinRange 5.0 1e+01) :!label _label_3) ; Wait a random amount of time (between\n5 and 10 seconds).
      (Audio|PlaySound2D "/Game/BoomToolkit/BoomDemo/Audio/Dialogue/Radio/A_BoomDemo_Radio_Mumble06_Cue.A_BoomDemo_Radio_Mumble06_Cue" 1.0 1.0 0.0 0 0) ; Play dialogue line.
      (Class|BPIntBoomDemoExample|TriggerMessage(Message) _returnvalue_2 "Dropping support in 3...2...1...") ; Trigger dialogue message.
      (Utilities|FlowControl|Delay 3.0) ; Wait 3 seconds.
      (Class|BPIntBoomDemoExample|TriggerMessage(Message) _returnvalue_2) ; Clear message.
      (Variables|Default|SetCurrentAssitance (Utilities|Array|Get(acopy) (Variables|Default|GetAssistanceActors) (Math|Random|RandomIntegerinRange 0 (Utilities|Array|LastIndex (Variables|Default|GetAssistanceActors))))) ; Randomize explosive actor for this run.
      (goto _label)
      (else
        (goto _label_2)))
    (else
      (goto _label_3))))

(fn ConstructionScript)

(fn BuildTransform
  (bind _box (Variables|Default|GetBox))
  (bind (_origin _boxextent) (Collision|GetComponentBounds _box))
  (bind _returnvalue (- _origin _boxextent))
  (bind _returnvalue_2 (+ _origin _boxextent))
  (bind (_x _y) (Math|Vector|BreakVector _returnvalue))
  (bind (_x_2 _y_2 _z) (Math|Vector|BreakVector _returnvalue_2))
  (return (Math|Transform|MakeTransform (Math|Vector|MakeVector (Math|Random|RandomFloatinRange _x_2 _x) (Math|Random|RandomFloatinRange _y_2 _y) _z) "-90.000000, 0, 0")))