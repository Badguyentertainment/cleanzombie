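; Demo button actor that lets an overlapping player fire a configurable projectile class from the button.
; Trigger overlap registers the button with the player and tints its dynamic material by usability.
; RunExample forwards to the server, which spawns the projectile with the player as owning pawn and instigator.
; The button then sinks, locks until a reset delay, and rises again, recoloring by whether the player still overlaps.
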(event OnComponentBeginOverlap(TriggerCollider)
  (params (OverlappedComponent :type Primitive%20Component%20Object%20Reference) (OtherActor :type Actor%20Object%20Reference) (OtherComp :type Primitive%20Component%20Object%20Reference) (OtherBodyIndex :type Integer) (bFromSweep :type Boolean) (SweepResult :type Hit%20Result%20Structure%20%28by%20ref%29))
  ;[1 1 1] Example projectil button logic.
  (bind _output_get (Variables|Default|SetPlayer OtherActor)) ; Store reference to overlapping player for use.
  (Class|BPIntBoomDemoExample|SetButton(Message) _output_get self) ; Update player reference to this actor.
  (if (Variables|Default|GetCanUse) ; Is the player allowed to use this actor?
    (Rendering|Material|SetVectorParameterValue (Variables|Default|GetButtonMaterial) "DiffuseColor" "(R=0.000000,G=1.000000,B=0.000000,A=1.000000)" :!class /Script/Engine.MaterialInstanceDynamic) ; Set button color to red.
    (else
      (Rendering|Material|SetVectorParameterValue (Variables|Default|GetButtonMaterial) "DiffuseColor" "(R=1.000000,G=0.000000,B=0.000000,A=1.000000)" :!class /Script/Engine.MaterialInstanceDynamic) ; Set button color to red.
    )))

(event OnComponentEndOverlap(TriggerCollider)
  (params (OverlappedComponent :type Primitive%20Component%20Object%20Reference) (OtherActor :type Actor%20Object%20Reference) (OtherComp :type Primitive%20Component%20Object%20Reference) (OtherBodyIndex :type Integer))
  ;[1 1 1] Example projectil button logic.
  (Class|BPIntBoomDemoExample|SetButton(Message) OtherActor) ; Clear player reference to this actor.
  (Rendering|Material|SetVectorParameterValue (Variables|Default|GetButtonMaterial) "DiffuseColor" "(R=0.000000,G=0.000000,B=1.000000,A=1.000000)" :!class /Script/Engine.MaterialInstanceDynamic) ; Set button color to red.
)

(event Custom|RunExample
  (bind _player (Variables|Default|GetPlayer))
  (bind _aspawn (Utilities|Casting|CastToPawn _player))
  ;[1 1 1] Example projectil button logic.
  (Networking|SwitchHasAuthority ; Are we running this on the server?
    (:Authority
      (if (Variables|Default|GetCanUse) ; Is the player allowed to use this actor?
        (Variables|Default|SetCanUse false) ; Stop player from using actor again until reset.
        (bind _returnvalue (Game|SpawnActorfromClass (Variables|Default|GetProjectileClass) (Math|Transform|MakeTransform (Transformation|GetWorldLocation (Variables|Default|GetScene)) "-90.000000, 0,0.000000") "Undefined" "SelectDefaultAtRuntime" 0 _aspawn _aspawn)) ; Spawn projectile class at location.
        (Class|BPBoomIntExplosionActor|SetOwningPawn(Message) _returnvalue _aspawn) ; Set owning pawn in projectlile to null reference.
        (Utilities|FlowControl|Sequence ; Do these in sequence...
          (:then_0
            (Rendering|Material|SetVectorParameterValue (Variables|Default|GetButtonMaterial) "DiffuseColor" "(R=1.000000,G=0.000000,B=0.000000,A=1.000000)" :!class /Script/Engine.MaterialInstanceDynamic) ; Set button color to red.
            (Components|MoveComponentTo (Variables|Default|GetStaticMesh) "0,0.000000,-100.000000" "0.000000, 0, 0" false false 0.5 false) ; Move mesh down 100 units over 0.5 seconds.
          )
          (:then_1
            (Utilities|FlowControl|Delay (Variables|Default|GetResetDelay)) ; Wait for the reset delay duration...
            (Components|MoveComponentTo (Variables|Default|GetStaticMesh) "0,0.000000,0.000000" "0.000000, 0, 0" false false 0.5 false) ; Return mesh to it's original location.
            (if (Collision|IsOverlappingActor (Variables|Default|GetTriggerCollider) (Variables|Default|GetPlayer) :!class /Script/Engine.PrimitiveComponent) ; Is the player that triggered this still overlapping the trigger?
              (Rendering|Material|SetVectorParameterValue (Variables|Default|GetButtonMaterial) "DiffuseColor" "(R=0.000000,G=1.000000,B=0.000000,A=1.000000)" :!class /Script/Engine.MaterialInstanceDynamic) ; Set button material back to green.
              (else
                (Rendering|Material|SetVectorParameterValue (Variables|Default|GetButtonMaterial) "DiffuseColor" "(R=0.000000,G=0.000000,B=1.000000,A=1.000000)" :!class /Script/Engine.MaterialInstanceDynamic) ; Set button color to blue.
              ))
            (Variables|Default|SetCanUse true) ; Reset use state for player to re-use.
          ))))
    (:Remote
      (CallFunction|ServerRunExample) ; Call this event on the server.
    )))

(event Custom|ServerRunExample
  (bind _player (Variables|Default|GetPlayer))
  (bind _aspawn (Utilities|Casting|CastToPawn _player))
  ;[1 1 1] Example projectil button logic.
  (Networking|SwitchHasAuthority ; Are we running this on the server?
    (:Authority
      (if (Variables|Default|GetCanUse) ; Is the player allowed to use this actor?
        (Variables|Default|SetCanUse false) ; Stop player from using actor again until reset.
        (bind _returnvalue (Game|SpawnActorfromClass (Variables|Default|GetProjectileClass) (Math|Transform|MakeTransform (Transformation|GetWorldLocation (Variables|Default|GetScene)) "-90.000000, 0,0.000000") "Undefined" "SelectDefaultAtRuntime" 0 _aspawn _aspawn)) ; Spawn projectile class at location.
        (Class|BPBoomIntExplosionActor|SetOwningPawn(Message) _returnvalue _aspawn) ; Set owning pawn in projectlile to null reference.
        (Utilities|FlowControl|Sequence ; Do these in sequence...
          (:then_0
            (Rendering|Material|SetVectorParameterValue (Variables|Default|GetButtonMaterial) "DiffuseColor" "(R=1.000000,G=0.000000,B=0.000000,A=1.000000)" :!class /Script/Engine.MaterialInstanceDynamic) ; Set button color to red.
            (Components|MoveComponentTo (Variables|Default|GetStaticMesh) "0,0.000000,-100.000000" "0.000000, 0, 0" false false 0.5 false) ; Move mesh down 100 units over 0.5 seconds.
          )
          (:then_1
            (Utilities|FlowControl|Delay (Variables|Default|GetResetDelay)) ; Wait for the reset delay duration...
            (Components|MoveComponentTo (Variables|Default|GetStaticMesh) "0,0.000000,0.000000" "0.000000, 0, 0" false false 0.5 false) ; Return mesh to it's original location.
            (if (Collision|IsOverlappingActor (Variables|Default|GetTriggerCollider) (Variables|Default|GetPlayer) :!class /Script/Engine.PrimitiveComponent) ; Is the player that triggered this still overlapping the trigger?
              (Rendering|Material|SetVectorParameterValue (Variables|Default|GetButtonMaterial) "DiffuseColor" "(R=0.000000,G=1.000000,B=0.000000,A=1.000000)" :!class /Script/Engine.MaterialInstanceDynamic) ; Set button material back to green.
              (else
                (Rendering|Material|SetVectorParameterValue (Variables|Default|GetButtonMaterial) "DiffuseColor" "(R=0.000000,G=0.000000,B=1.000000,A=1.000000)" :!class /Script/Engine.MaterialInstanceDynamic) ; Set button color to blue.
              ))
            (Variables|Default|SetCanUse true) ; Reset use state for player to re-use.
          ))))
    (:Remote
      (CallFunction|ServerRunExample) ; Call this event on the server.
    )))

(event EventBeginPlay
  ;[1 1 1] Example projectil button logic.
  (bind _returnvalue (Rendering|Material|CreateDynamicMaterialInstance (Variables|Default|GetStaticMesh) 1 "/Game/BoomToolkit/BoomDemo/Materials/MI_BoomDemo_ButtonMaterial.MI_BoomDemo_ButtonMaterial" "None" :!class /Script/Engine.PrimitiveComponent)) ; Get a reference to the button's dynamic material.
  (Variables|Default|SetButtonMaterial _returnvalue) ; Store reference for future use.
)

(fn ConstructionScript)