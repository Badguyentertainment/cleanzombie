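; Boom Toolkit actor for explosion after effects, combining configurable particle, mesh, sound, post-process and radial damage over time for a set lifetime.
; Multicast Initialize applies visuals on all machines, optionally growing the particle via a timer-driven VInterp, while only the server runs the damage loop.
; Multicast KillActor fades particle and sound, then the server either expires the actor or destroys effect components, leaving a persistent, optionally physics-simulated mesh.
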(event Custom|Initialize
  ;[1 1 1] Custom Boom Toolkit Events.
  ;;[0.5 0.5 0] Initialize Multicast - Initialize after effects actor.
  (CallFunction|InitializeEffect) ; Initialize AfterEffectsActor.
)

(event Custom|KillActor
  ;[1 1 1] Custom Boom Toolkit Events.
  ;;[0.5 0.5 0] KillActor Multicast - Process death of after effects actor.
  (CallFunction|ProcessDeath))

(fn ConstructionScript
  (Physics|SetSimulatePhysics (Variables|Data|GetStaticMesh) (Variables|SoundAndVisuals|GetMakePhysicsObject)) ; Update object physics state.
  (Class|PrimitiveComponent|SetMassOverrideinKg (Variables|Data|GetStaticMesh) "None" (Variables|SoundAndVisuals|GetObjectMass) true) ; Update object mass.
)

(fn InitializeEffect
  (Transformation|AddActorLocalOffset (Math|Vector|MakeVector 0.0 0.0 (Variables|Settings|GetHeightOffset)) false false) ; Add any height offset to this actor.
  (if (Variables|Settings|GetInheritRotation) ; Do we want to maintain the rotation parsed from the explosion?
    _
    (else
      (Transformation|SetActorRotation "0, 0, 0") ; Reset rotation.
    ))
  (Utilities|IsValid (Variables|SoundAndVisuals|GetParticleEffect) ; Is this actor set to use a valid particle effect?
    (:Is%20Valid
      ;[1 1 1] Initialize particle effect.
      (Effects|Components|ParticleSystem|SetTemplate (Variables|Data|GetParticleSystem) (Variables|SoundAndVisuals|GetParticleEffect)) ; Set the after effect particle.
      (if (Variables|SoundAndVisuals|GetScaleUpParticle) ; Do we want to scale the particle over time?
        (Transformation|SetRelativeScale3D (Variables|Data|GetParticleSystem) "0.100000,0.100000,0.100000") ; Set starting scale for particle to 0.1.
        (Components|Activation|Activate (Variables|Data|GetParticleSystem) false) ; Activate particle effect.
        (Utilities|Time|SetTimerbyFunctionName 0 "ScaleUp" 0.01 true) ; Start particle scale up loop.
        (else
          (Transformation|SetRelativeScale3D (Variables|Data|GetParticleSystem) (Math|Conversions|ToVector(Float) (Variables|SoundAndVisuals|GetTargetScale))) ; Set particle scale to target.
          (Components|Activation|Activate (Variables|Data|GetParticleSystem) false) ; Activate particle effect.
        )))
    (:Is%20Not%20Valid
      _))
  (Utilities|IsValid (Variables|SoundAndVisuals|GetMesh) ; Is this actor set to use a valid static mesh?
    (:Is%20Valid
      ;[1 1 1] Initialize static mesh.
      (Components|StaticMesh|SetStaticMesh (Variables|Data|GetStaticMesh) (Variables|SoundAndVisuals|GetMesh)) ; Set the after effect static mesh.
    )
    (:Is%20Not%20Valid
      _))
  (Utilities|IsValid (Variables|SoundAndVisuals|GetEffectSound) ; Make sure the sound parsed is valid.
    (:Is%20Valid
      ;[1 1 1] Initialize sound.
      (bind _returnvalue (Audio|SpawnSoundAttached (Variables|SoundAndVisuals|GetEffectSound) (Variables|Data|GetParticleSystem) "None" "0, 0, 0" "0, 0, 0" "KeepRelativeOffset" false 0.1 1.0 0.0 "/Game/BoomToolkit/Blueprints/Data/SA_Boom_Default.SA_Boom_Default" 0)) ; Spawn sound for particle effect.
      (bind _output_get (Variables|Data|SetActiveSound _returnvalue)) ; Store sound as variable for later\ncancelation.
      (Utilities|IsValid _output_get ; Is the active sound still valid?
        (:Is%20Valid
          (Audio|Components|Audio|FadeIn (Variables|Data|GetActiveSound) 1.0 1e+01 0.0 "Linear" :!class /Script/Engine.AudioComponent) ; Fade sound from spawn volume (0.1) to full.
        )
        (:Is%20Not%20Valid
          _)))
    (:Is%20Not%20Valid
      _))
  (Components|Sphere|SetSphereRadius (Variables|Data|GetEffectRadius) (Variables|Damage|GetDamageRadius) true) ; Update effect radius.
  (Networking|SwitchHasAuthority ; Ensure remainder of initialize only occurs\non server.
    (:Authority
      (if (and (Variables|Damage|GetCauseDamage) (!= (Variables|Damage|GetDamageRate) 0.0)) ; Should this actor cause damage to others\nAND is the damage amount set to a value\nother than zero?
        (Utilities|Time|SetTimerbyFunctionName 0 "DamageOverTime" (Variables|Damage|GetDamageFrequency) true) ; Start damage over time loop.
      ))
    (:Remote
      _))
  (Variables|/Script/Engine.PostProcessComponent|SetSettings (Variables|Data|GetPostProcess) (Variables|SoundandVisuals|GetPostProcessing)) ; Set post processing settings.
  (Utilities|Time|SetTimerbyFunctionName 0 "KillActor" (Variables|Settings|GetLifetime)) ; Set timer for kill actor.
  (return) ; Done.
)

(fn ScaleUp
  (bind _particlesystem (Variables|Data|GetParticleSystem))
  (bind _returnvalue (Transformation|GetWorldScale _particlesystem))
  (Transformation|SetRelativeScale3D (Variables|Data|GetParticleSystem) (Math|Interpolation|VInterpTo _returnvalue (Math|Conversions|ToVector(Float) (Variables|SoundAndVisuals|GetTargetScale)) 0.025 1.0)) ; Update the particle effect scale by the\nVInterp amount.
  (if (Math|Vector|Equal(Vector) _returnvalue (Math|Conversions|ToVector(Float) (Variables|SoundAndVisuals|GetTargetScale)) 0.0001) ; Has the VInterp hit the target scale?
    (Utilities|Time|ClearTimerbyFunctionName 0 "ScaleUp") ; Stop the scale up loop.
    (return) ; Done.
    (else
      (return) ; Done.
    )))

(fn DamageOverTime
  (for _array_element (Collision|GetOverlappingActors (Variables|Data|GetEffectRadius) "/Script/Engine.Actor" :!class /Script/Engine.PrimitiveComponent) ; For every actor in range...
    (Game|Damage|ApplyDamage _array_element (Variables|Damage|GetDamageRate) (Game|GetInstigatorController) (Variables|Damage|GetCauser) (Variables|Damage|GetDamageType)) ; Apply the damage amount per cycle.
  )
  (return) ; Done.
)

(fn KillAfterEffect
  (Utilities|Time|ClearTimerbyFunctionName 0 "DamageOverTime") ; Stop damage over time cycle.
  (if (Variables|Settings|GetPersistentMesh) ; Is this after effect set to have a persistent mesh?
    (Utilities|Time|SetTimerbyFunctionName 0 "KillEffect" (Variables|Settings|GetDeactivationTime)) ; Set a timer for KillEffect, killing the particle system, post\nprocessing component and effect radius component after\nthe deactivation time, but allowing the mesh to remain.
    (return) ; Done.
    (else
      (Actor|SetLifeSpan (Variables|Settings|GetDeactivationTime)) ; Set actor lifetime, using Deactivation\nTime to allow for particle to correctly\ndeactivate visually.
      (return) ; Done.
    )))

(fn ProcessDeath
  (Components|Activation|Deactivate (Variables|Data|GetParticleSystem)) ; Deactivate particle effect.
  (Utilities|IsValid (Variables|Data|GetActiveSound) ; Is there a valid active sound?
    (:Is%20Valid
      (Audio|Components|Audio|FadeOut (Variables|Data|GetActiveSound) (Variables|Settings|GetDeactivationTime) 0.0 "Linear" :!class /Script/Engine.AudioComponent) ; Fade sound over deactivation period.
    )
    (:Is%20Not%20Valid
      _))
  (Networking|SwitchHasAuthority ; Ensure the remainder of KillActor event\nonly runs on network authority (server).
    (:Authority
      (CallFunction|KillAfterEffect) ; Kill AfterEffectsActor.
      (return) ; Done
    )
    (:Remote
      (return) ; Done
    )))

(fn KillEffect
  (Components|DestroyComponent (Variables|Data|GetParticleSystem)))